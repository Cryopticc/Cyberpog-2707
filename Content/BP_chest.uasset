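; Interactable chest that the player opens by holding interact until a progress bar fills.
; Overlap shows or hides a SearchWidget, interact begin and end drive its progress, and a delegate is bound to the bar filling.
; OpenChest hides the widget, plays a timeline to pitch the lid, turns on a light and spawns two Niagara effects.
; A Closed macro gates all interaction once opened.
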(event `self.ReceiveBeginPlay`
  (bind _assearch_widget (cast `/Game/SearchWidget` (`WidgetComponent.GetUserWidgetObject` (`self.Widget`))))
  (set `/Game/SearchWidget.Progress % Speed` 2.0 _assearch_widget)
  (add `/Game/SearchWidget.OnProgressBarFull` _assearch_widget (`|CreateDelegate` :!event `OpenChest`)))

(event `/Game/Interact_Interface.OnOverlapBegin`
  (`self.Closed`
    (:`true`
      (`SceneComponent.SetVisibility` (`self.Widget`) true false))))

(event `/Game/Interact_Interface.OnOverlapEnd`
  (`self.Closed`
    (:`true`
      (`SceneComponent.SetVisibility` (`self.Widget`) false false))))

(event `/Game/Interact_Interface.OnInteractBegin`
  (`self.Closed`
    (:`true`
      (bind _assearch_widget (cast `/Game/SearchWidget` (`WidgetComponent.GetUserWidgetObject` (`self.Widget`))))
      (`/Game/SearchWidget.BeginProgress` _assearch_widget))))

(event `/Game/Interact_Interface.OnInteractEnd`
  (`self.Closed`
    (:`true`
      (bind _assearch_widget (cast `/Game/SearchWidget` (`WidgetComponent.GetUserWidgetObject` (`self.Widget`))))
      (`/Game/SearchWidget.EndProgress` _assearch_widget))))

(fn `OpenChest`
  (bind _returnvalue (`self.K2_GetActorLocation`))
  (`self.Closed`
    (:`true`
      (set `self.Open?` true)
      (`SceneComponent.SetVisibility` (`self.Widget`) false false)
      (`TimelineComponent.PlayFromStart` (`self.Open Chest Timeline`))
      (`SceneComponent.SetVisibility` (`self.PointLight`) true false)
      (`NiagaraFunctionLibrary.SpawnSystemAtLocation` "/Game/NS_Chest_open.NS_Chest_open" _returnvalue)
      (`NiagaraFunctionLibrary.SpawnSystemAtLocation` "/Game/NS_Chest_open2.NS_Chest_open2" _returnvalue))))

(fn `UserConstructionScript`)